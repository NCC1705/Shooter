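; Molten Grux beetle enemy Blueprint that supplies the UI side of combat: a health bar and floating hit numbers.
; On BeginPlay it links the health bar widget to itself and hides it, then show and hide events toggle its visibility.
; Each hit spawns a HitNumber widget at the screen-projected hit location, registers it through StoreHitNumber, and displays the damage with a headshot flag.
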(event `self.ReceiveBeginPlay`
  ;[1 1 1] Super::BeginPlay();
  (`parent.ReceiveBeginPlay`)
  (bind _asenemy_health_bar_bp (cast `/Game/_Game/HUD/EnemyHealthBarBP` (`WidgetComponent.GetUserWidgetObject` (`self.HealthBarWidget`))))
  (set `/Game/_Game/HUD/EnemyHealthBarBP.Enemy` self _asenemy_health_bar_bp)
  (`Widget.SetVisibility` (`WidgetComponent.GetUserWidgetObject` (`self.HealthBarWidget`)) "Hidden"))

(event `self.ShowHealthBar`
  (`Widget.SetVisibility` (`WidgetComponent.GetUserWidgetObject` (`self.HealthBarWidget`)) "Visible")
  (`parent.ShowHealthBar`))

(event `self.HideHealthBar`
  (`Widget.SetVisibility` (`WidgetComponent.GetUserWidgetObject` (`self.HealthBarWidget`)) "Hidden"))

(event `self.ShowHitNumber`
  (params (Damage :type Integer) (HitLocation :type "Vector Structure") (bHeadShot :type Boolean))
  (bind _returnvalue (`|CreateWidget` "/Game/_Game/HUD/HitNumber.HitNumber_C"))
  (`UserWidget.AddToViewport` _returnvalue 0)
  (`UserWidget.SetPositionInViewport` _returnvalue (`GameplayStatics.ProjectWorldToScreen` (`GameplayStatics.GetPlayerController` 0) HitLocation) true)
  (`self.StoreHitNumber` _returnvalue HitLocation)
  (`/Game/_Game/HUD/HitNumber.Display` _returnvalue Damage bHeadShot))

(fn `UserConstructionScript`)